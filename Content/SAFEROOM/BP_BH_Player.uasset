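; BP_BH_Player is a player actor that moves on the X-Z plane and shoots bullets.
; Tick calls Movement_2, which offsets location by the move axes times MoveSpeed, without sweep, delta time or any real bounds check; the older Movement function is unused.
; Interact or Space Bar spawns a BP_Bullet 500 units along world +X, copying the player's rotation and scale.
; Overlaps only print a hit message.
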(event `self.ReceiveTick`
  (params (DeltaSeconds :type "Float (single-precision)"))
  (bind _returnvalue (`KismetMathLibrary.MakeVector` (+ (* (`self.moveSpeed`) (`self.GetInputAxisValue`)) (.x (`self.K2_GetActorLocation`))) (.y (`self.K2_GetActorLocation`)) (+ (.z (`self.K2_GetActorLocation`)) (* (`self.GetInputAxisValue`) (`self.moveSpeed`)))))
  (set `self.deltaSeconds` DeltaSeconds)
  (set `self.moveToLoc` _returnvalue)
  (if true
    (`self.K2_SetActorLocation` _returnvalue)))

(event `self.ReceiveActorBeginOverlap`
  (params (OtherActor :type "Actor Object Reference"))
  (`KismetSystemLibrary.PrintString` "Player: OUCH!"))

(event `InputAction|Interact`
  (params (Key :type "Key Structure"))
  ;[1 1 1] Press E (or space bar) to shoot
  (:`Pressed`
    (`|SpawnActorFromClass` "/Game/SAFEROOM/BP_Bullet.BP_Bullet_C" (`KismetMathLibrary.MakeTransform` (+ (.location (`self.GetTransform`)) (500.0 0.0 0.0)) (.rotation (`self.GetTransform`)) (.scale (`self.GetTransform`))) "Undefined" "OverrideRootScale" null null :!label _label)))

(event `Key|SpaceBar`
  (params (Key :type "Key Structure"))
  (:`Pressed`
    (goto _label)))

(fn `UserConstructionScript`)