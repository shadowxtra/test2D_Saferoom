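; Button Blueprint for SAFEROOM menus that keeps mouse hover and keyboard focus in sync visually.
; Start launches a looping timer that polls CheckFocus ten times a second.
; When hovered, the button takes user focus, applies the mouse style and prints a debug string.
; Otherwise it switches between selected and unselected key styles based on keyboard focus.
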(fn `CheckFocus`
  (if (`self.IsHovered`)
    (`self.SetUserFocus` null)
    (`self.SetStyle` (`self.MouseStyle`))
    (`KismetSystemLibrary.PrintString` "CheckFocus is Fiering")
    (else
      (`self.SetStyle` (select `bool` (`self.HasKeyboardFocus`) :`false` (`self.KeyNotSelected`) :`true` (`self.KeySelected`))))))

(fn `Start`
  (`KismetSystemLibrary.K2_SetTimer` null "CheckFocus" 0.1 true))