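; BP_BH_Enemy is an enemy actor that fires bullets at a regular interval and loses health when touched.
; Tick accumulates play time and calls ShootForward whenever SecondsPerShot has elapsed since the last shot.
; ShootForward spawns a BP_Bullet at a fixed world-space offset along negative X, rotated 180 degrees, and sets its sprite.
; Any actor overlap subtracts fixed HP and prints debug messages, with no death handling.
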(event `self.ReceiveTick`
  (params (DeltaSeconds :type "Float (single-precision)"))
  (bind _output_get (set `self.secondsPlayed` (+ (stale _output_get) DeltaSeconds)))
  (if (> (- _output_get (`self.lastShotTime`)) (`self.SecondsPerShot`))
    (set `self.lastShotTime` _output_get)
    (`self.Shoot forward`)))

(event `self.ReceiveActorBeginOverlap`
  (params (OtherActor :type "Actor Object Reference"))
  (`KismetSystemLibrary.PrintString` "Enemy: OUCH!")
  (bind _output_get (set `self.HP` (- (stale _output_get) 20.0)))
  (`KismetSystemLibrary.PrintString` (`KismetStringLibrary.Concat_StrStr` "HP: " (`KismetStringLibrary.Conv_DoubleToString` _output_get) "%")))

(event `Shoot forward`
  ;[1 1 1] ??? to shoot
  (bind _returnvalue (`|SpawnActorFromClass` "/Game/SAFEROOM/BP_Bullet.BP_Bullet_C" (`KismetMathLibrary.MakeTransform` (+ (.location (`self.GetTransform`)) (-500.0 0.0 0.0)) (struct :`Yaw` 180.0) (.scale (`self.GetTransform`))) "Undefined" "OverrideRootScale" null null))
  (`/Game/SAFEROOM/BP_Bullet.setSprite` _returnvalue 1))

(fn `UserConstructionScript`)