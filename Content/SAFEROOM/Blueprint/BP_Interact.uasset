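; Interactable actor that shows and hides a dialogue box on screen, displaying its own MyText.
; Interact toggles the widget: it removes an existing one, or creates one for player 0, adds it to the viewport and sets its text.
; An end-overlap handler closes and clears the widget when the 2DSideScrollerCharacter leaves, after a validity check.
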(event `/Game/SAFEROOM/Blueprint/Interact_Interface.Interact`
  (`/Engine/EditorBlueprintResources/StandardMacros.IsValid` (`self.DialougeWidget`)
    (:`Is Valid`
      (`Widget.RemoveFromParent` (`self.DialougeWidget`))
      (set `self.DialougeWidget` null))
    (:`Is Not Valid`
      (bind _returnvalue (`|CreateWidget` "/Game/SAFEROOM/Dialouge/DialougeWidget.DialougeWidget_C" (`GameplayStatics.GetPlayerController` 0)))
      (bind _output_get (set `self.DialougeWidget` _returnvalue))
      (`UserWidget.AddToViewport` _output_get 0)
      (set `/Game/SAFEROOM/Dialouge/DialougeWidget.DialougeText` (`self.MyText`) (`self.DialougeWidget`)))))

(event `OnComponentEndOverlap_Event_0`
  (params (OverlappedComponent :type "PrimitiveComponent Object Reference") (OtherActor :type "Actor Object Reference") (OtherComp :type "PrimitiveComponent Object Reference") (OtherBodyIndex :type Integer))
  (`/Engine/EditorBlueprintResources/StandardMacros.IsValid` null
    (:`Is Valid`
      (cast `/Game/SAFEROOM/Blueprint/Player/2DSideScrollerCharacter` OtherActor)
      (`Widget.RemoveFromParent` (`self.DialougeWidget`))
      (set `self.DialougeWidget` null))))

(fn `UserConstructionScript`)