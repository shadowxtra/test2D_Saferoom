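; BP_Pendulum is an actor that swings like a pendulum by rotating itself around its pitch axis.
; On BeginPlay it caches its starting rotation, starts the PendulumSwing timeline and sets that timeline's play rate from SwingSpeed.
; Each timeline update multiplies the Rotation track by SwingDistanceDegrees and adds it to the original pitch, keeping roll and yaw at their starting values.
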(event `self.ReceiveBeginPlay`
  (set `self.OriginalRotation` (`self.K2_GetActorRotation`))
  (`self.StartPendulumSwing`)
  (`TimelineComponent.SetPlayRate` (`self.PendulumSwing`) (`self.SwingSpeed`)))

(event `StartPendulumSwing`
  (bind (_originalrotation_roll _originalrotation_pitch _originalrotation_yaw) (`KismetMathLibrary.BreakRotator` (`self.OriginalRotation`)))
  (bind (_direction _rotation) (`Timeline|PendulumSwing`)
    (:`Update`
      (`self.K2_SetActorRotation` (`KismetMathLibrary.MakeRotator` _originalrotation_roll (+ _originalrotation_pitch (* _rotation (`self.SwingDistanceDegrees`))) _originalrotation_yaw)))))

(fn `UserConstructionScript`)