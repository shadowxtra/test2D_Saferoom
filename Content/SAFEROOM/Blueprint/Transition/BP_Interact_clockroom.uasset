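; Interactable transition actor that sends the player to the ClockRoom_LVL level when its Interact event fires.
; Construction script writes ObjectName into a TextRender label.
; Each tick it measures the distance to the player character and shows the label only within a fixed radius, hiding it otherwise.
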(event `self.ReceiveTick`
  (params (DeltaSeconds :type "Float (single-precision)"))
  (bind _textrender (`self.TextRender`))
  (if (< (`KismetMathLibrary.VSize` (- (`self.K2_GetActorLocation` (`GameplayStatics.GetPlayerCharacter` 0)) (`self.K2_GetActorLocation`))) 500.0)
    (`SceneComponent.SetVisibility` _textrender true false)
    (else
      (`SceneComponent.SetVisibility` _textrender false false))))

(event `/Game/SAFEROOM/Blueprint/Interact_Interface.Interact`
  (`GameplayStatics.OpenLevel` "ClockRoom_LVL"))

(fn `UserConstructionScript`
  (`TextRenderComponent.K2_SetText` (`self.TextRender`) (`self.ObjectName`)))