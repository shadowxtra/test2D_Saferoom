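; Actor component that continuously spins its owning actor around selected world axes.
; Each Tick, RotateOwner scales RotationSpeed by delta time to get a frame-rate-independent rotation step.
; The RotateX, RotateY and RotateZ flags each gate a separate world rotation for roll, pitch and yaw, so any combination of axes can spin at the same shared speed.
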(event `self.ReceiveTick`
  (params (DeltaSeconds :type "Float (single-precision)"))
  (`self.RotateOwner` DeltaSeconds))

(fn `RotateOwner`
  (params (DeltaSeconds :type "Float (double-precision)"))
  (locals (RotationToAdd :type "Rotator Structure"))
  (bind _returnvalue (`self.GetOwner`))
  (bind (_rotationtoadd_roll _rotationtoadd_pitch _rotationtoadd_yaw) (`KismetMathLibrary.BreakRotator` (`local.RotationToAdd`)))
  (bind _returnvalue_2 (* DeltaSeconds (`self.RotationSpeed`)))
  (set `local.RotationToAdd` (`KismetMathLibrary.MakeRotator` _returnvalue_2 _returnvalue_2 _returnvalue_2))
  (`|ExecutionSequence`
    (:`then_0`
      (if (`self.RotateX`)
        (`Actor.K2_AddActorWorldRotation` _returnvalue (`KismetMathLibrary.MakeRotator` _rotationtoadd_roll) false false)))
    (:`then_1`
      (if (`self.RotateY`)
        (`Actor.K2_AddActorWorldRotation` _returnvalue (`KismetMathLibrary.MakeRotator` 0.0 _rotationtoadd_pitch) false false)))
    (:`then_2`
      (if (`self.RotateZ`)
        (`Actor.K2_AddActorWorldRotation` _returnvalue (`KismetMathLibrary.MakeRotator` 0.0 0.0 _rotationtoadd_yaw) false false)))))