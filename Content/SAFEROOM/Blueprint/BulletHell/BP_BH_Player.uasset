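; Player pawn for a bullet hell game, moving on the X/Z plane through axis-driven movement input.
; Interact or Space spawns a BP_Bullet offset along world +X, and Escape quits the game.
; Any actor overlap decrements PlayerHealth in MyGameInstance, resetting it and opening Saferoom_Test_2 at zero.
; A manual SetActorLocation movement function remains, but its call in the event graph never runs.
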(event `InputAxis|MoveRight`
  (params (AxisValue :type "Float (single-precision)"))
  ;[1 1 1] movement
  (`self.AddMovementInput` (1.0 0.0 0.0) AxisValue))

(event `self.ReceiveTick`
  (params (DeltaSeconds :type "Float (single-precision)"))
  (set `self.deltaSeconds` DeltaSeconds))

(event `InputAxis|MoveForward`
  (params (AxisValue :type "Float (single-precision)"))
  ;[1 1 1] movement
  (`self.AddMovementInput` (0.0 0.0 1.0) AxisValue))

(event `Key|Escape`
  (params (Key :type "Key Structure"))
  (:`Pressed`
    (`KismetSystemLibrary.QuitGame` null "Quit")))

(event `self.ReceiveActorBeginOverlap`
  (params (OtherActor :type "Actor Object Reference"))
  ;[1 1 1] take damage
  (`KismetSystemLibrary.PrintString` "Player: OUCH!")
  (bind _asmy_game_instance (cast `/Game/SAFEROOM/Blueprint/Transition/MyGameInstance` (`GameplayStatics.GetGameInstance`)))
  (bind _output_get (set `/Game/SAFEROOM/Blueprint/Transition/MyGameInstance.PlayerHealth` (- (stale _output_get) 1) _asmy_game_instance))
  ;[1 1 1] if player dies
  (if (<= _output_get 0)
    (set `/Game/SAFEROOM/Blueprint/Transition/MyGameInstance.PlayerHealth` 3 _asmy_game_instance)
    (`GameplayStatics.OpenLevel` "Saferoom_Test_2")))

(event `InputAction|Interact`
  (params (Key :type "Key Structure"))
  ;[1 1 1] Press E (or space bar) to shoot
  (:`Pressed`
    (`|SpawnActorFromClass` "/Game/SAFEROOM/Blueprint/BulletHell/BP_Bullet.BP_Bullet_C" (`KismetMathLibrary.MakeTransform` (+ (.location (`self.GetTransform`)) (500.0 0.0 0.0)) (.rotation (`self.GetTransform`)) (.scale (`self.GetTransform`))) "Undefined" "OverrideRootScale" null null :!label _label)))

(event `Key|SpaceBar`
  (params (Key :type "Key Structure"))
  (:`Pressed`
    (goto _label)))

(fn `UserConstructionScript`)