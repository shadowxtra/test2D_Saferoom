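; Bullet actor for the bullet hell game, with a selectable paper sprite (arrow or enemy attack) and movement behavior.
; Each tick it teleport-free moves along its forward vector, either straight or slower with a time-driven sine wave on Z around its spawn height.
; Movement uses a fixed per-frame step without sweep or delta-time scaling.
; It destroys itself shortly after any actor overlap.
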(event `setSprite`
  (params (look :type Integer))
  ;[1 1 1] set sprite lok
  (switch `int` look
    (:`0`
      (`PaperSpriteComponent.SetSprite` (`self.PaperSprite`) "/Game/SAFEROOM/SPRITES/BulletHell_Sprites/BH_temp_Arrow_Sprite.BH_temp_Arrow_Sprite"))
    (:`1`
      (`PaperSpriteComponent.SetSprite` (`self.PaperSprite`) "/Game/SAFEROOM/SPRITES/BulletHell_Sprites/BH_temp_EnemyAttack_Sprite.BH_temp_EnemyAttack_Sprite"))))

(event `self.ReceiveBeginPlay`
  ;[1 1 1] beginPlay: set Original Z value
  (set `self.originalZ` (.z (`SceneComponent.K2_GetComponentLocation` (`self.DefaultSceneRoot`)))))

(event `set behavior`
  (params (`Behavior type` :type Integer))
  ;[1 1 1] function: set behavior
  (set `self.myBehaviorType` `Behavior type`))

(event `self.ReceiveActorBeginOverlap`
  (params (OtherActor :type "Actor Object Reference"))
  ;[1 1 1] destroy self after any collision
  (`KismetSystemLibrary.Delay` 0.01)
  (`self.K2_DestroyActor`))

(event `self.ReceiveTick`
  (params (DeltaSeconds :type "Float (single-precision)"))
  ;[1 1 1] track time (for wave movement)
  (bind _output_get (set `self.secondsSinceSpawn` (+ (stale _output_get) DeltaSeconds)))
  ;[1 1 1] which behavior to follow
  (switch `int` (`self.myBehaviorType`)
    (:`0`
      (set `self.moveSpeed` 25.0)
      ;[1 1 1] behavor type 0: move forward
      (`self.K2_SetActorLocation` (+ (`self.K2_GetActorLocation`) (* (`self.GetActorForwardVector`) (`self.moveSpeed`)))))
    (:`1`
      (set `self.moveSpeed` 10.0)
      ;[1 1 1] behavor type 1: move forward with sine wave
      (`self.K2_SetActorLocation` (`KismetMathLibrary.MakeVector` (.x (+ (`self.K2_GetActorLocation`) (* (`self.GetActorForwardVector`) (`self.moveSpeed`)))) (.y (+ (`self.K2_GetActorLocation`) (* (`self.GetActorForwardVector`) (`self.moveSpeed`)))) (+ (`self.originalZ`) (* (`KismetMathLibrary.DegSin` (* (`self.secondsSinceSpawn`) 260.0)) 1000.0)))))))

(fn `UserConstructionScript`)