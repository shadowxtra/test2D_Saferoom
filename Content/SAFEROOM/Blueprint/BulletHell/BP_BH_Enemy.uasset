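; BP_BH_Enemy is the enemy in a bullet-hell game, firing bullets and losing health when hit.
; At BeginPlay it randomly picks one of two attack types, each setting bullet look, behavior and fire interval.
; Tick accumulates play time and spawns a BP_BH_Bullet at an X offset whenever the interval elapses, passing it sprite and behavior.
; Any actor overlap subtracts a fixed amount from EnemyHealth on BP_BulletHell_GameMode and prints debug text.
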(event `set attack type`
  (params (`attack type` :type Integer))
  ;[1 1 1] function: set attack type
  (bind _output_get (set `self.activeAttackType` `attack type`))
  (switch `int` _output_get
    (:`Default`
      (set `self.Bullet_look` 0 :!label _label)
      (set `self.Bullet_behavior` 0)
      (set `self.SecondsPerShot` 0.5))
    (:`0`
      (goto _label))
    (:`1`
      (set `self.Bullet_look` 1)
      (set `self.Bullet_behavior` 1)
      (set `self.SecondsPerShot` 1.3))))

(event `self.ReceiveTick`
  (params (DeltaSeconds :type "Float (single-precision)"))
  (bind _output_get (set `self.secondsPlayed` (+ (stale _output_get) DeltaSeconds)))
  ;[1 1 1] call attack function
  (`self.Shoot function`))

(event `self.ReceiveBeginPlay`
  (`self.set attack type` (`KismetMathLibrary.RandomIntegerInRange` 0 1)))

(event `self.ReceiveActorBeginOverlap`
  (params (OtherActor :type "Actor Object Reference"))
  ;[1 1 1] get hit = take damage
  (`KismetSystemLibrary.PrintString` "Enemy: OUCH!")
  (bind _asbp_bullet_hell_game_mode (cast `/Game/SAFEROOM/Blueprint/BulletHell/BP_BulletHell_GameMode` (`GameplayStatics.GetGameMode`)))
  (bind _output_get (set `/Game/SAFEROOM/Blueprint/BulletHell/BP_BulletHell_GameMode.enemyHealth` (- (stale _output_get) (`self.HP_lossPercentPerHit`)) _asbp_bullet_hell_game_mode))
  (`KismetSystemLibrary.PrintString` (`KismetStringLibrary.Concat_StrStr` "HP: " (`KismetStringLibrary.Conv_DoubleToString` _output_get) "%")))

(event `Shoot function`
  (bind _secondsplayed (`self.secondsPlayed`))
  ;[1 1 1] function: shoot
  ;;[1 1 1] check if time to attack
  (if (> (- _secondsplayed (`self.lastShotTime`)) (`self.SecondsPerShot`))
    (set `self.lastShotTime` _secondsplayed)
    ;;[1 1 1] shoot
    (bind _returnvalue (`|SpawnActorFromClass` "/Game/SAFEROOM/Blueprint/BulletHell/BP_BH_Bullet.BP_BH_Bullet_C" (`KismetMathLibrary.MakeTransform` (+ (.location (`self.GetTransform`)) (-500.0 0.0 0.0)) (struct :`Yaw` 180.0) (.scale (`self.GetTransform`))) "Undefined" "OverrideRootScale" null null))
    (`/Game/SAFEROOM/Blueprint/BulletHell/BP_BH_Bullet.setSprite` _returnvalue (`self.Bullet_look`))
    (`/Game/SAFEROOM/Blueprint/BulletHell/BP_BH_Bullet.set behavior` _returnvalue (`self.Bullet_behavior`))))

(fn `UserConstructionScript`)