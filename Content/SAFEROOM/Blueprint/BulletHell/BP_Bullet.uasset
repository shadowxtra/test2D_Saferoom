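; BP_Bullet is a bullet-hell projectile with a switchable sprite that destroys itself on overlapping non-bullet actors, or when the game mode is paused.
; Each Tick advances a spawn timer and moves it by behavior type: fast straight flight, or named variants (Sw1, Sw2, Depression, Jealousy, Anxiety).
; These variants move forward through near-duplicate SineWave helpers, meant to oscillate Z around the height recorded at BeginPlay.
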(event `setSprite`
  (params (look :type Integer))
  ;[1 1 1] set sprite look
  (switch `int` look
    (:`Default`
      (`PaperSpriteComponent.SetSprite` (`self.PaperSprite`) (`self.BasicEnemyBullet`) :!label _label)
      (`SceneComponent.SetRelativeScale3D` (`self.PaperSprite`) (1.0 1.0 1.0)))
    (:`0`
      (goto _label))
    (:`1`
      (`PaperSpriteComponent.SetSprite` (`self.PaperSprite`) (`self.EnemyTypeSprite`)))))

(event `self.ReceiveBeginPlay`
  ;[1 1 1] beginPlay: set Original Z value
  (set `self.originalZ` (.z (`SceneComponent.K2_GetComponentLocation` (`self.DefaultSceneRoot`)))))

(event `set behavior`
  (params (`Behavior type` :type Integer))
  ;[1 1 1] function: set behavior
  (set `self.myBehaviorType` `Behavior type`))

(event `self.ReceiveActorBeginOverlap`
  (params (OtherActor :type "Actor Object Reference"))
  ;[1 1 1] destroy self after any collision (except other bullets)
  (cast `/Game/SAFEROOM/Blueprint/BulletHell/BP_Bullet` OtherActor
    (:`CastFailed`
      (`KismetSystemLibrary.Delay` 0.01)
      (`self.K2_DestroyActor`))))

(event `self.ReceiveTick`
  (params (DeltaSeconds :type "Float (single-precision)"))
  ;[1 1 1] destroy if game is paused
  (bind _asbp_bullet_hell_game_mode (cast `/Game/SAFEROOM/Blueprint/BulletHell/BP_BulletHell_GameMode` (`GameplayStatics.GetGameMode`)))
  (if (`/Game/SAFEROOM/Blueprint/BulletHell/BP_BulletHell_GameMode.gameIsPaused` _asbp_bullet_hell_game_mode)
    (`self.K2_DestroyActor`)
    (else
      (set `self.Delta Seconds` DeltaSeconds)
      ;[1 1 1] track time (for wave movement)
      (bind _output_get (set `self.secondsSinceSpawn` (+ (stale _output_get) DeltaSeconds)))
      ;[1 1 1] which behavior to follow
      (switch `int` (`self.myBehaviorType`)
        (:`0`
          (set `self.moveSpeed` 2500.0)
          ;[1 1 1] behavor type 0: move forward
          (`self.K2_SetActorLocation` (+ (`self.K2_GetActorLocation`) (* (`self.GetActorForwardVector`) (* (`self.moveSpeed`) (`self.Delta Seconds`))))))
        (:`1`
          (set `self.moveSpeed` 500.0)
          (`self.K2_SetActorLocation` (`KismetMathLibrary.MakeVector` (.x (+ (`self.K2_GetActorLocation`) (* (`self.GetActorForwardVector`) (* (`self.moveSpeed`) (`self.Delta Seconds`))))) (.y (+ (`self.K2_GetActorLocation`) (* (`self.GetActorForwardVector`) (* (`self.moveSpeed`) (`self.Delta Seconds`))))) (+ (`self.originalZ`) (* (`KismetMathLibrary.DegSin` (* 100.0 (`self.secondsSinceSpawn`))) 800.0)))))
        (:`2`
          (set `self.moveSpeed` 500.0)
          (`self.K2_SetActorLocation` (`KismetMathLibrary.MakeVector` (.x (+ (`self.K2_GetActorLocation`) (* (`self.GetActorForwardVector`) (* (`self.moveSpeed`) (`self.Delta Seconds`))))) (.y (+ (`self.K2_GetActorLocation`) (* (`self.GetActorForwardVector`) (* (`self.moveSpeed`) (`self.Delta Seconds`))))) (+ (`self.originalZ`) (* (`KismetMathLibrary.DegSin` (* 100.0 (`self.secondsSinceSpawn`))) 800.0)))))
        (:`3`
          (set `self.moveSpeed` 500.0)
          (`self.K2_SetActorLocation` (`KismetMathLibrary.MakeVector` (.x (+ (`self.K2_GetActorLocation`) (* (`self.GetActorForwardVector`) (* (`self.moveSpeed`) (`self.Delta Seconds`))))) (.y (+ (`self.K2_GetActorLocation`) (* (`self.GetActorForwardVector`) (* (`self.moveSpeed`) (`self.Delta Seconds`))))) (+ (`self.originalZ`) (* (`KismetMathLibrary.DegSin` (* 100.0 (`self.secondsSinceSpawn`))) 800.0)))))
        (:`4`
          (set `self.moveSpeed` 500.0)
          (`self.K2_SetActorLocation` (`KismetMathLibrary.MakeVector` (.x (+ (`self.K2_GetActorLocation`) (* (`self.GetActorForwardVector`) (* (`self.moveSpeed`) (`self.Delta Seconds`))))) (.y (+ (`self.K2_GetActorLocation`) (* (`self.GetActorForwardVector`) (* (`self.moveSpeed`) (`self.Delta Seconds`))))) (+ (`self.originalZ`) (* (`KismetMathLibrary.DegSin` (* 100.0 (`self.secondsSinceSpawn`))) 800.0)))))
        (:`5`
          (set `self.moveSpeed` 1000.0)
          (`self.K2_SetActorLocation` (`KismetMathLibrary.MakeVector` (.x (+ (`self.K2_GetActorLocation`) (* (`self.GetActorForwardVector`) (* (`self.moveSpeed`) (`self.Delta Seconds`))))) (.y (+ (`self.K2_GetActorLocation`) (* (`self.GetActorForwardVector`) (* (`self.moveSpeed`) (`self.Delta Seconds`))))) (+ (`self.originalZ`) (* (`KismetMathLibrary.DegSin` (* 100.0 (`self.secondsSinceSpawn`))) 800.0)))))))))

(fn `UserConstructionScript`)