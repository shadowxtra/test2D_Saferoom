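; Game mode for the bullet hell minigame that switches between fight-or-flight menu, active combat and ended states.
; The menu event adds a button widget, shows the cursor and focuses the buttons.
; Starting a fight clears the widget, unpauses, hides the cursor and sets a countdown, shorter when fleeing, which also disables the player's shooting.
; Ending a fight only flags the game as paused and not fighting.
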(event `endFighting`
  (set `self.gameIsPaused` true)
  (set `self.isFighting` false))

(event `fightOrFlightMenu`
  (`|ExecutionSequence`
    (:`then_0`
      (bind _returnvalue (`|CreateWidget` "/Game/SAFEROOM/Menus/BulletHell_ButtonWidget.BulletHell_ButtonWidget_C"))
      (`UserWidget.AddToViewport` _returnvalue 0))
    (:`then_1`
      (set `PlayerController.bShowMouseCursor` true (`GameplayStatics.GetPlayerController` 0))
      (set `self.showFightFlightButtons` true)
      (`/Game/SAFEROOM/Menus/BulletHell_ButtonWidget.setFocusOnButtons` (`self.widget`)))))

(event `startFight`
  (`Widget.RemoveFromParent` (`self.widget`))
  (set `self.gameIsPaused` false)
  (set `self.isFighting` true)
  (set `self.showFightFlightButtons` false)
  (set `PlayerController.bShowMouseCursor` false (`GameplayStatics.GetPlayerController` 0))
  ;[1 1 1] set countdown time
  (if (`self.isFlighting`)
    (set `self.fightCountdown` 5.0)
    (bind _asbp_bh_player (cast `/Game/SAFEROOM/Blueprint/BulletHell/BP_BH_Player` (`GameplayStatics.GetPlayerPawn` 0)))
    (set `/Game/SAFEROOM/Blueprint/BulletHell/BP_BH_Player.canShoot` false _asbp_bh_player)
    (else
      (set `self.fightCountdown` 10.0))))

(fn `UserConstructionScript`)