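; Base enemy for bullet-hell encounters, framing combat rounds with dialogue and a fight-or-flight menu through BP_BulletHell_GameMode.
; While unpaused, Tick moves it vertically at random speed, fires timed BP_Bullets and runs down the round countdown.
; Countdown expiry either completes a flight or reopens the menu, alternating two attack patterns.
; Overlaps drain health, triggering dialogue at half and zero; defeat is recorded in MyGameInstance before loading the return level.
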(event `self.ReceiveTick`
  (params (DeltaSeconds :type "Float (single-precision)"))
  (set `self.Delta Seconds` DeltaSeconds)
  ;[1 1 1] check that game isn't paused
  (bind _asbp_bullet_hell_game_mode (cast `/Game/SAFEROOM/Blueprint/BulletHell/BP_BulletHell_GameMode` (`GameplayStatics.GetGameMode`)))
  (if (not (`/Game/SAFEROOM/Blueprint/BulletHell/BP_BulletHell_GameMode.gameIsPaused` _asbp_bullet_hell_game_mode))
    (bind _output_get (set `self.secondsPlayed` (+ (stale _output_get) DeltaSeconds)))
    (`self.move about`)
    (`self.Shoot function`)
    ;[1 1 1] is fight over
    (bind _asbp_bullet_hell_game_mode_2 (cast `/Game/SAFEROOM/Blueprint/BulletHell/BP_BulletHell_GameMode` (`GameplayStatics.GetGameMode`)))
    (bind _output_get_2 (set `/Game/SAFEROOM/Blueprint/BulletHell/BP_BulletHell_GameMode.fightCountdown` (- (stale _output_get_2) DeltaSeconds) _asbp_bullet_hell_game_mode_2))
    (if (<= (`/Game/SAFEROOM/Blueprint/BulletHell/BP_BulletHell_GameMode.fightCountdown` _asbp_bullet_hell_game_mode_2) 0.0)
      (if (`/Game/SAFEROOM/Blueprint/BulletHell/BP_BulletHell_GameMode.isFlighting` _asbp_bullet_hell_game_mode_2)
        ;[1 1 1] successful flight
        (bind _asbp_bullet_hell_game_mode_3 (cast `/Game/SAFEROOM/Blueprint/BulletHell/BP_BulletHell_GameMode` (`GameplayStatics.GetGameMode`)))
        (`/Game/SAFEROOM/Blueprint/BulletHell/BP_BulletHell_GameMode.endFighting` _asbp_bullet_hell_game_mode_3)
        ;[1 1 1] dialogue
        (bind _returnvalue (`|AddComponentByClass` "/Game/SAFEROOM/Dialouge/BPC_Dialogue.BPC_Dialogue_C" "/Game/SAFEROOM/Dialouge/DT_GameDialogue.DT_GameDialogue" "flightSuccess"))
        (`/Game/SAFEROOM/Dialouge/BPC_Dialogue.OnActivate` _returnvalue (delegate `endDialogue3`))
        (else
          ;[1 1 1] pause in fight
          (bind _asbp_bullet_hell_game_mode_4 (cast `/Game/SAFEROOM/Blueprint/BulletHell/BP_BulletHell_GameMode` (`GameplayStatics.GetGameMode`)))
          (`/Game/SAFEROOM/Blueprint/BulletHell/BP_BulletHell_GameMode.endFighting` _asbp_bullet_hell_game_mode_4)
          ;;[1 1 1] dialogue
          (bind _returnvalue_2 (`|AddComponentByClass` "/Game/SAFEROOM/Dialouge/BPC_Dialogue.BPC_Dialogue_C" "/Game/SAFEROOM/Dialouge/DT_GameDialogue.DT_GameDialogue" "fight_or_flight"))
          (`/Game/SAFEROOM/Dialouge/BPC_Dialogue.OnActivate` _returnvalue_2 (delegate `CustomEvent`)))))))

(event `endDialogue3`
  ;[1 1 1] dialogue
  (`GameplayStatics.OpenLevel` (`self.ReturnToLevel`)))

(event `CustomEvent`
  ;[1 1 1] dialogue
  ;[1 1 1] pause in fight
  (`/Game/SAFEROOM/Blueprint/BulletHell/BP_BulletHell_GameMode.fightOrFlightMenu` (stale `self.ReceiveTick` _asbp_bullet_hell_game_mode_4))
  ;[1 1 1] switch attack type
  (`/Engine/EditorBlueprintResources/StandardMacros.FlipFlop`
    (:`A`
      (`self.set attack type` 1))
    (:`B`
      (`self.set attack type` 0))))

(event `self.ReceiveBeginPlay`
  ;[1 1 1] initial tag types
  (`self.set attack type` 0)
  (`PaperSpriteComponent.SetSprite` (`self.PaperSprite`) (`self.Enemy_Sprite`))
  (bind _asbp_bullet_hell_game_mode (cast `/Game/SAFEROOM/Blueprint/BulletHell/BP_BulletHell_GameMode` (`GameplayStatics.GetGameMode`)))
  (`/Game/SAFEROOM/Blueprint/BulletHell/BP_BulletHell_GameMode.endFighting` _asbp_bullet_hell_game_mode)
  ;[1 1 1] welcome dialogue
  (bind _returnvalue (`|AddComponentByClass` "/Game/SAFEROOM/Dialouge/BPC_Dialogue.BPC_Dialogue_C" "/Game/SAFEROOM/Dialouge/DT_GameDialogue.DT_GameDialogue" (`self.DialogueName_welcome`)))
  (`/Game/SAFEROOM/Dialouge/BPC_Dialogue.OnActivate` _returnvalue (delegate `welcomeDialogueEnded`)))

(event `welcomeDialogueEnded`
  ;[1 1 1] welcome dialogue
  (bind _asbp_bullet_hell_game_mode (cast `/Game/SAFEROOM/Blueprint/BulletHell/BP_BulletHell_GameMode` (`GameplayStatics.GetGameMode`)))
  (`/Game/SAFEROOM/Blueprint/BulletHell/BP_BulletHell_GameMode.fightOrFlightMenu` _asbp_bullet_hell_game_mode))

(event `set attack type`
  (params (`attack type` :type Integer))
  ;[1 1 1] function: set attack type
  (bind _output_get (set `self.activeAttackType` `attack type`))
  (switch `int` _output_get
    (:`Default`
      (set `self.Bullet_look` 0 :!label _label)
      (set `self.Bullet_behavior` 1)
      (set `self.SecondsPerShot` 1.3))
    (:`0`
      (set `self.Bullet_look` 1)
      (set `self.Bullet_behavior` 0)
      (set `self.SecondsPerShot` 0.5))
    (:`1`
      (goto _label))))

(event `endDialogue`
  ;[1 1 1] if low health: dialogue (then fight/flight)
  (`/Game/SAFEROOM/Blueprint/BulletHell/BP_BulletHell_GameMode.fightOrFlightMenu` (stale `self.ReceiveActorBeginOverlap` _asbp_bullet_hell_game_mode_3)))

(event `self.ReceiveActorBeginOverlap`
  (params (OtherActor :type "Actor Object Reference"))
  ;[1 1 1] get hit = take damage
  (bind _asbp_bullet_hell_game_mode (cast `/Game/SAFEROOM/Blueprint/BulletHell/BP_BulletHell_GameMode` (`GameplayStatics.GetGameMode`)))
  (bind _output_get (set `/Game/SAFEROOM/Blueprint/BulletHell/BP_BulletHell_GameMode.enemyHealth` (- (stale _output_get) (`self.HP_lossPercentPerHit`)) _asbp_bullet_hell_game_mode))
  (switch `int` (`self.dialoguesHad`)
    (:`Default`
      ;[1 1 1] if defeated: dialogue
      (if (<= _output_get 0.0) :!label _label_2
        (bind _asbp_bullet_hell_game_mode_2 (cast `/Game/SAFEROOM/Blueprint/BulletHell/BP_BulletHell_GameMode` (`GameplayStatics.GetGameMode`)))
        (`/Game/SAFEROOM/Blueprint/BulletHell/BP_BulletHell_GameMode.endFighting` _asbp_bullet_hell_game_mode_2)
        (bind _returnvalue (`|AddComponentByClass` "/Game/SAFEROOM/Dialouge/BPC_Dialogue.BPC_Dialogue_C" "/Game/SAFEROOM/Dialouge/DT_GameDialogue.DT_GameDialogue" (`self.DialogueName_noHealth`)))
        (`/Game/SAFEROOM/Dialouge/BPC_Dialogue.OnActivate` _returnvalue (delegate `endDialogue2`))))
    (:`0`
      ;[1 1 1] if low health: dialogue (then fight/flight)
      (if (<= _output_get 50.0)
        (bind _output_get_2 (set `self.dialoguesHad` (+ (stale _output_get_2) 1)))
        (bind _asbp_bullet_hell_game_mode_3 (cast `/Game/SAFEROOM/Blueprint/BulletHell/BP_BulletHell_GameMode` (`GameplayStatics.GetGameMode`)))
        (`/Game/SAFEROOM/Blueprint/BulletHell/BP_BulletHell_GameMode.endFighting` _asbp_bullet_hell_game_mode_3)
        (bind _returnvalue_2 (`|AddComponentByClass` "/Game/SAFEROOM/Dialouge/BPC_Dialogue.BPC_Dialogue_C" "/Game/SAFEROOM/Dialouge/DT_GameDialogue.DT_GameDialogue" (`self.DialogueName_halfHealth`)))
        (`/Game/SAFEROOM/Dialouge/BPC_Dialogue.OnActivate` _returnvalue_2 (delegate `endDialogue`))))
    (:`1`
      (goto _label_2))))

(event `Shoot function`
  (bind _secondsplayed (`self.secondsPlayed`))
  ;[1 1 1] function: shoot
  ;;[1 1 1] check if time to attack
  (if (> (- _secondsplayed (`self.lastShotTime`)) (`self.SecondsPerShot`))
    (set `self.lastShotTime` _secondsplayed)
    ;;[1 1 1] shoot
    (bind _returnvalue (`|SpawnActorFromClass` "/Game/SAFEROOM/Blueprint/BulletHell/BP_Bullet.BP_Bullet_C" (`KismetMathLibrary.MakeTransform` (+ (.location (`self.GetTransform`)) (-500.0 0.0 0.0)) (struct :`Yaw` 180.0) (.scale (`self.GetTransform`))) "Undefined" "OverrideRootScale" null null))
    (`/Game/SAFEROOM/Blueprint/BulletHell/BP_Bullet.setSprite` _returnvalue (`self.Bullet_look`))
    (`/Game/SAFEROOM/Blueprint/BulletHell/BP_Bullet.set behavior` _returnvalue (`self.Bullet_behavior`))))

(event `endDialogue2`
  ;[1 1 1] if defeated: dialogue
  ;[1 1 1] + set enemy to defeated + return to hub
  (bind _asmy_game_instance (cast `/Game/SAFEROOM/Blueprint/Transition/MyGameInstance` (`GameplayStatics.GetGameInstance`)))
  (`KismetArrayLibrary.Array_Set` (`/Game/SAFEROOM/Blueprint/Transition/MyGameInstance.EnemiesDefeated` _asmy_game_instance) (`self.myEncounter_ID`) true)
  (`GameplayStatics.OpenLevel` (`self.ReturnToLevel`)))

(fn `move about`
  (locals (bounds_top :type "Float (double-precision)" :default 800.0) (movementSpeed :type "Float (double-precision)" :default 10.0))
  (bind _defaultsceneroot (`self.DefaultSceneRoot`))
  (bind _defaultsceneroot_2 (`self.DefaultSceneRoot`))
  (bind (_returnvalue_x _returnvalue_y _returnvalue_z) (`KismetMathLibrary.BreakVector` (`SceneComponent.K2_GetComponentLocation` _defaultsceneroot)))
  (bind (_returnvalue_x_2 _returnvalue_y_2 _returnvalue_z_2) (`KismetMathLibrary.BreakVector` (`SceneComponent.K2_GetComponentLocation` _defaultsceneroot_2)))
  (bind _returnvalue (- _returnvalue_z_2 (`local.movementSpeed`)))
  (bind _returnvalue_2 (+ _returnvalue_z (`local.movementSpeed`)))
  (set `local.movementSpeed` (`KismetMathLibrary.RandomFloatInRange` 5.0 20.0))
  (if (`self.isMovingUp`)
    (`SceneComponent.K2_SetWorldLocation` _defaultsceneroot_2 (`KismetMathLibrary.MakeVector` _returnvalue_x_2 _returnvalue_y_2 _returnvalue) false false)
    (if (>= (`KismetMathLibrary.Abs` _returnvalue) (`local.bounds_top`))
      (set `self.isMovingUp` false))
    (else
      (`SceneComponent.K2_SetWorldLocation` _defaultsceneroot (`KismetMathLibrary.MakeVector` _returnvalue_x _returnvalue_y _returnvalue_2) false false)
      (if (>= (`KismetMathLibrary.Abs` _returnvalue_2) (`local.bounds_top`))
        (set `self.isMovingUp` true)))))

(fn `UserConstructionScript`)