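; BFL_Helpers is a Blueprint helper library that tracks per-NPC dialogue progress, counting times talked.
; A shared getter casts the Game Instance to MyGameInstance, whose DialogueProgressMap holds the counts keyed by NPC name.
; Get, Set and Increment functions read and write that map, treating a missing NPC as zero.
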(fn `Get MyGameInstance`
  (returns (MyGameInstance :type "/Game/SAFEROOM/Blueprint/Transition/MyGameInstance Object Reference"))
  (bind _asmy_game_instance (cast `/Game/SAFEROOM/Blueprint/Transition/MyGameInstance` (`GameplayStatics.GetGameInstance` null))
    (:`then`
      (return _asmy_game_instance))
    (:`CastFailed`
      (return null))))

(fn `GetDialogueProgress`
  (params (NPC_Name :type Name))
  (returns (TimesTalked :type Integer))
  (bind (_value _returnvalue) (`BlueprintMapLibrary.Map_Find` (`/Game/SAFEROOM/Blueprint/Transition/MyGameInstance.DialogueProgressMap` (`self.Get MyGameInstance` null)) NPC_Name))
  (if _returnvalue
    (return _value)
    (else
      (return 0))))

(fn `IncrementDialogueProgress`
  (params (NPC_Name :type Name))
  (returns (TimesTalked :type Integer))
  (bind _dialogueprogressmap (`/Game/SAFEROOM/Blueprint/Transition/MyGameInstance.DialogueProgressMap` (`self.Get MyGameInstance` null)))
  (bind (_value _returnvalue) (`BlueprintMapLibrary.Map_Find` _dialogueprogressmap NPC_Name))
  (bind _returnvalue_2 (select `bool` _returnvalue :`false` 1 :`true` (+ _value 1)))
  (`BlueprintMapLibrary.Map_Add` _dialogueprogressmap NPC_Name _returnvalue_2)
  (return _returnvalue_2))

(fn `SetDialogueProgress`
  (params (NPC_Name :type Name) (NewTimesTalked :type "Integer (by ref)"))
  (`BlueprintMapLibrary.Map_Add` (`/Game/SAFEROOM/Blueprint/Transition/MyGameInstance.DialogueProgressMap` (`self.Get MyGameInstance` null)) NPC_Name NewTimesTalked))