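; BPC_Dialogue is a component that shows a speaker's dialogue in an on-screen box while locking player movement.
; On activation it looks up a row in its data table, replaces any open W_Dialogue_Box with a new one, and passes it the speaker, lines, symbol delay and completion callback.
; OnFinished unlocks BP_Player movement and destroys the component, making it single-use.
; A missing table or row prints an error.
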(fn `ChangeMovementLock`
  (params (LockMovement :type Boolean))
  (bind _asbp_player (cast `/Game/SAFEROOM/Blueprint/Player/BP_Player` (`GameplayStatics.GetPlayerPawn` 0)))
  (set `/Game/SAFEROOM/Blueprint/Player/BP_Player.LockMovement` LockMovement _asbp_player))

(fn `OnActivate`
  (params (OnDialogueCompletion :type "Delegate (by ref)"))
  (bind _rowname (`self.RowName`))
  (`/Engine/EditorBlueprintResources/StandardMacros.IsValid` (`self.DialogueTable`)
    (:`Is Valid`
      (bind _returnvalue (`|GetDataTableRow` (`self.DialogueTable`) _rowname)
        (:`then`
          (`self.ChangeMovementLock` true)
          (bind _foundwidgets (`WidgetBlueprintLibrary.GetAllWidgetsOfClass` "/Game/SAFEROOM/Dialouge/W_Dialogue_Box.W_Dialogue_Box_C"))
          (for _array_element _foundwidgets
            (`Widget.RemoveFromParent` _array_element))
          (bind _returnvalue_2 (`|CreateWidget` "/Game/SAFEROOM/Dialouge/W_Dialogue_Box.W_Dialogue_Box_C" (`GameplayStatics.GetPlayerController` 0)))
          (bind (_speakername _dialoguetext) (break `/Game/SAFEROOM/Dialouge/Struct_Dialogue` _returnvalue))
          (`/Game/SAFEROOM/Dialouge/W_Dialogue_Box.InitializeWidget` _returnvalue_2 self _speakername _dialoguetext (`self.Text Symbol Delay`) OnDialogueCompletion)
          (`UserWidget.AddToViewport` _returnvalue_2 1000))
        (:`RowNotFound`
          (`KismetSystemLibrary.PrintString` (`KismetStringLibrary.Concat_StrStr` "BPC_Dialogue ERROR: No row found with the name \"" (`KismetStringLibrary.Conv_NameToString` _rowname) "\"") true true (struct :`R` 1.0 :`A` 1.0) 10.0))))
    (:`Is Not Valid`
      (`KismetSystemLibrary.PrintString` "BPC_Dialogue ERROR: No data table set in \"Dialogue Table\"" true true (struct :`R` 1.0 :`A` 1.0) 10.0))))

(fn `OnFinished`
  (`self.ChangeMovementLock` false)
  (`self.K2_DestroyComponent`))